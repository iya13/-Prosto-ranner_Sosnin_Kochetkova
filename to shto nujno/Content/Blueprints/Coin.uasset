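; Coin pickup actor, built from Недорубль cube, cylinder and text components, that disappears when the ThirdPersonCharacter touches it.
; Each part's overlap casts the other actor to ThirdPersonCharacter and destroys the coin, but only the cylinder also plays the money sound at the character's location.
; An InstancedStaticMesh overlap plays that sound at world origin without destroying the actor.
; No score is updated, and a leftover sound chain is unconnected.
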(event `self.недорубль_Cube.OnComponentBeginOverlap`
  (params (OverlappedComponent :type "PrimitiveComponent Object Reference") (OtherActor :type "Actor Object Reference") (OtherComp :type "PrimitiveComponent Object Reference") (OtherBodyIndex :type Integer) (bFromSweep :type Boolean) (SweepResult :type "HitResult Structure (by ref)"))
  (cast `/Game/ThirdPersonBP/Blueprints/ThirdPersonCharacter` OtherActor)
  (`self.K2_DestroyActor`))

(event `self.недорубль_Cylinder.OnComponentBeginOverlap`
  (params (OverlappedComponent :type "PrimitiveComponent Object Reference") (OtherActor :type "Actor Object Reference") (OtherComp :type "PrimitiveComponent Object Reference") (OtherBodyIndex :type Integer) (bFromSweep :type Boolean) (SweepResult :type "HitResult Structure (by ref)"))
  (bind _asthird_person_character (cast `/Game/ThirdPersonBP/Blueprints/ThirdPersonCharacter` OtherActor))
  (`self.K2_DestroyActor`)
  (`GameplayStatics.PlaySoundAtLocation` "/Game/Runner/upali-dengi-na-igrovoy-schet.upali-dengi-na-igrovoy-schet" (`self.K2_GetActorLocation` _asthird_person_character) (struct) 1.0 1.0 0.0 null null null))

(event `self.недорубль_Text.OnComponentBeginOverlap`
  (params (OverlappedComponent :type "PrimitiveComponent Object Reference") (OtherActor :type "Actor Object Reference") (OtherComp :type "PrimitiveComponent Object Reference") (OtherBodyIndex :type Integer) (bFromSweep :type Boolean) (SweepResult :type "HitResult Structure (by ref)"))
  (cast `/Game/ThirdPersonBP/Blueprints/ThirdPersonCharacter` OtherActor)
  (`self.K2_DestroyActor`))

(event `self.InstancedStaticMesh.OnComponentBeginOverlap`
  (params (OverlappedComponent :type "PrimitiveComponent Object Reference") (OtherActor :type "Actor Object Reference") (OtherComp :type "PrimitiveComponent Object Reference") (OtherBodyIndex :type Integer) (bFromSweep :type Boolean) (SweepResult :type "HitResult Structure (by ref)"))
  (cast `/Game/ThirdPersonBP/Blueprints/ThirdPersonCharacter` OtherActor)
  (`GameplayStatics.PlaySoundAtLocation` "/Game/Runner/upali-dengi-na-igrovoy-schet.upali-dengi-na-igrovoy-schet" (0.0 0.0 0.0) (struct) 1.0 1.0 0.0 null null null))

(fn `UserConstructionScript`)