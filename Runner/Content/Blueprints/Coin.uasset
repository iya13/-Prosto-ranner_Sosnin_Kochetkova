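; Coin pickup actor that the third-person character collects by touching it, and that destroys itself 60 seconds after BeginPlay if left alone.
; Actor overlap and StaticMesh overlap each increment Coins on ThirdPersonGameMode, play a 2D sound and destroy the coin.
; Separate overlap handlers on the Недорубль Cube, Cylinder and Text components destroy it without adding coins, with only the Cylinder playing the sound, at the character's location.
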(event `self.ReceiveBeginPlay`
  (`KismetSystemLibrary.Delay` 60.0)
  (`self.K2_DestroyActor`))

(event `self.ReceiveActorBeginOverlap`
  (params (OtherActor :type "Actor Object Reference"))
  (cast `/Game/ThirdPersonBP/Blueprints/ThirdPersonCharacter` OtherActor)
  (bind _asthird_person_game_mode (cast `/Game/ThirdPersonBP/Blueprints/ThirdPersonGameMode` (`GameplayStatics.GetGameMode`)))
  (`/Engine/EditorBlueprintResources/StandardMacros.IncrementInt` (`/Game/ThirdPersonBP/Blueprints/ThirdPersonGameMode.Coins` _asthird_person_game_mode)
    (:`  `
      (`GameplayStatics.SpawnSound2D` "/Game/Runner/upali-dengi-na-igrovoy-schet.upali-dengi-na-igrovoy-schet" 1.0 1.0 0.0 null)
      (`self.K2_DestroyActor`))))

(event `self.недорубль_Cube.OnComponentBeginOverlap`
  (params (OverlappedComponent :type "PrimitiveComponent Object Reference") (OtherActor :type "Actor Object Reference") (OtherComp :type "PrimitiveComponent Object Reference") (OtherBodyIndex :type Integer) (bFromSweep :type Boolean) (SweepResult :type "HitResult Structure (by ref)"))
  (cast `/Game/ThirdPersonBP/Blueprints/ThirdPersonCharacter` OtherActor)
  (`self.K2_DestroyActor`))

(event `self.недорубль_Cylinder.OnComponentBeginOverlap`
  (params (OverlappedComponent :type "PrimitiveComponent Object Reference") (OtherActor :type "Actor Object Reference") (OtherComp :type "PrimitiveComponent Object Reference") (OtherBodyIndex :type Integer) (bFromSweep :type Boolean) (SweepResult :type "HitResult Structure (by ref)"))
  (bind _asthird_person_character (cast `/Game/ThirdPersonBP/Blueprints/ThirdPersonCharacter` OtherActor))
  (`self.K2_DestroyActor`)
  (`GameplayStatics.PlaySoundAtLocation` "/Game/Runner/upali-dengi-na-igrovoy-schet.upali-dengi-na-igrovoy-schet" (`self.K2_GetActorLocation` _asthird_person_character) (struct) 1.0 1.0 0.0 null null null))

(event `self.недорубль_Text.OnComponentBeginOverlap`
  (params (OverlappedComponent :type "PrimitiveComponent Object Reference") (OtherActor :type "Actor Object Reference") (OtherComp :type "PrimitiveComponent Object Reference") (OtherBodyIndex :type Integer) (bFromSweep :type Boolean) (SweepResult :type "HitResult Structure (by ref)"))
  (cast `/Game/ThirdPersonBP/Blueprints/ThirdPersonCharacter` OtherActor)
  (`self.K2_DestroyActor`))

(event `self.StaticMesh.OnComponentBeginOverlap`
  (params (OverlappedComponent :type "PrimitiveComponent Object Reference") (OtherActor :type "Actor Object Reference") (OtherComp :type "PrimitiveComponent Object Reference") (OtherBodyIndex :type Integer) (bFromSweep :type Boolean) (SweepResult :type "HitResult Structure (by ref)"))
  (cast `/Game/ThirdPersonBP/Blueprints/ThirdPersonCharacter` OtherActor)
  (bind _asthird_person_game_mode (cast `/Game/ThirdPersonBP/Blueprints/ThirdPersonGameMode` (`GameplayStatics.GetGameMode`)))
  (`/Engine/EditorBlueprintResources/StandardMacros.IncrementInt` (`/Game/ThirdPersonBP/Blueprints/ThirdPersonGameMode.Coins` _asthird_person_game_mode)
    (:`  `
      (`GameplayStatics.SpawnSound2D` "/Game/Runner/upali-dengi-na-igrovoy-schet.upali-dengi-na-igrovoy-schet" 1.0 1.0 0.0 null)
      (`self.K2_DestroyActor`))))

(fn `UserConstructionScript`)